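; Lobby game mode that names joining players and moves the session to the chosen level once everyone is ready.
; PostLogin gives each player state a numbered "User" nickname, and BeginPlay enables seamless travel.
; TryStartGame checks every player's Ready flag, then runs a ServerTravel console command built from LevelName.
; SaveConfig sets LevelName and writes clamped counts to the game instance, with the bot count overwriting MaxPlayerCount.
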(event Custom|TryStartGame
  ;[0.15 0.15 0.15 0.5] Try StartGame
  (if (CallFunction|IsEverybodyReady)
    (Development|ExecuteConsoleCommand (Utilities|String|Append "ServerTravel" " " (Variables|Default|GetLevelName)) 0)))

(event EventPostLogin
  (params (NewPlayer :type Player%20Controller%20Object%20Reference))
  (bind _nicknameindex (Variables|Default|GetNicknameIndex))
  ;[0.15 0.15 0.15 0.5] Set Nickname
  (bind _asbp_lobby_player_state (Utilities|Casting|CastToBP_LobbyPlayerState (Variables|/Script/Engine.Controller|GetPlayerState NewPlayer)))
  (Math|Integer|IncrementInt _nicknameindex
    (:%20%20
      (Variables|/Game/Blueprints/Lobby/BP_LobbyPlayerState.BP_LobbyPlayerState_C|SetNickname _asbp_lobby_player_state (Utilities|Text|FormatText "User{0}" _nicknameindex)))))

(event EventBeginPlay
  ;[0.15 0.15 0.15 0.5] Seamless Travel
  (Variables|Default|SetbUseSeamlessTravel true))

(fn ConstructionScript)

(fn IsEverybodyReady
  ;[0.15 0.15 0.15 0.5] IsEverybodyReady
  (for _array_element (Variables|/Script/Engine.GameStateBase|GetPlayerArray (Game|GetGameState))
    (bind _asbp_lobby_player_state (Utilities|Casting|CastToBP_LobbyPlayerState _array_element))
    (if (not (Variables|/Game/Blueprints/Lobby/BP_LobbyPlayerState.BP_LobbyPlayerState_C|GetReady _asbp_lobby_player_state))
      (return false)))
  (return true))

(fn SaveConfig
  (params (InLevelName :type String) (InMaxPlayerCount :type Integer) (InMaxBotCount :type Integer))
  ;[0.15 0.15 0.15 0.5] Save Config
  (Utilities|FlowControl|Sequence
    (:then_0
      (bind _asbp_game_instance (Utilities|Casting|CastToBP_GameInstance (Game|GetGameInstance)))
      (Variables|Default|SetBPGameInstance _asbp_game_instance))
    (:then_1
      (switch string InLevelName
        (:Fountain
          (Variables|Default|SetLevelName "Level_Fountain"))
        (:Watermill
          (Variables|Default|SetLevelName "Level_Watermill"))))
    (:then_2
      (Variables|/Game/Blueprints/BP_GameInstance.BP_GameInstance_C|SetMaxPlayerCount (Variables|Default|GetBPGameInstance) (Math|Integer|Clamp(Integer) InMaxPlayerCount 2 10)))
    (:then_3
      (Variables|/Game/Blueprints/BP_GameInstance.BP_GameInstance_C|SetMaxPlayerCount (Variables|Default|GetBPGameInstance) (Math|Integer|Clamp(Integer) InMaxBotCount 10 30)))))