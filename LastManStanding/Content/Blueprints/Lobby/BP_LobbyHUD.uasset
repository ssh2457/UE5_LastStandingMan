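; BP_LobbyHUD is a lobby HUD Blueprint that creates and owns the lobby screen UI.
; On BeginPlay it creates a WBP_Lobby widget, adds it to the viewport, and for a local player controller switches to UI-only input with the mouse cursor shown.
; Its RefreshUI event forwards to the widget's own refresh when the widget is valid.
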(event Custom|RefreshUI
  (bind _lobbyui (Variables|Default|GetLobbyUI))
  ;[0.15 0.15 0.15 0.5] Refresh UI
  (Utilities|IsValid _lobbyui
    (:Is%20Valid
      (Default|RefreshUI _lobbyui))))

(event EventBeginPlay
  (bind _returnvalue (Game|GetPlayerController 0))
  ;[0.15 0.15 0.15 0.5] Create Lobby UI
  (bind _returnvalue_2 (UserInterface|CreateWidget "/Game/Assets/UI/Widgets/Lobby/WBP_Lobby.WBP_Lobby_C"))
  (bind _output_get (Variables|Default|SetLobbyUI _returnvalue_2))
  (UserInterface|Viewport|AddtoViewport _output_get 0)
  (if (Pawn|IsLocalPlayerController _returnvalue)
    (Input|SetInputModeUIOnly _returnvalue 0 "DoNotLock" false)
    (Variables|/Script/Engine.PlayerController|SetbShowMouseCursor _returnvalue true)))

(fn ConstructionScript)