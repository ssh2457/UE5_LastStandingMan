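; BP_LobbyPlayerState is the lobby PlayerState, holding each player's nickname and ready flag.
; Spawn, destruction, the ready multicast and nickname replication all refresh the local player's lobby HUD.
; CopyProperties carries the nickname into BP_PlayerState, and a client kick event opens the Title level.
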(event Custom|OnDestroyed_Event
  (params (DestroyedActor :type Actor%20Object%20Reference))
  (CallFunction|RefreshLobbyUI))

(event Custom|Multicast_Ready
  ;[0.15 0.15 0.15 0.5] Set Ready
  (Variables|Default|SetReady true)
  (CallFunction|RefreshLobbyUI))

(event Custom|Client_KickedByServer
  ;[0.15 0.15 0.15 0.5] Kicked By Server
  (Game|OpenLevel(byObjectReference) "/Game/Maps/Title.Title"))

(event EventCopyProperties
  (params (NewPlayerState :type Player%20State%20Object%20Reference))
  ;[0.15 0.15 0.15 0.5] CopyProperties
  (|CallParentFunction NewPlayerState)
  (bind _asbp_player_state (Utilities|Casting|CastToBP_PlayerState NewPlayerState))
  (Variables|/Game/Blueprints/Game/Characters/Player/BP_PlayerState.BP_PlayerState_C|SetNickname _asbp_player_state (Variables|Default|GetNickname)))

(event EventBeginPlay
  (CallFunction|RefreshLobbyUI)
  (Game|AssignOnDestroyed (delegate Custom|OnDestroyed_Event)))

(fn ConstructionScript)

(fn RefreshLobbyUI
  (bind _returnvalue (Game|GetPlayerController 0))
  ;[0.15 0.15 0.15 0.5] Refresh Lobby UI
  (Utilities|IsValid _returnvalue
    (:Is%20Valid
      (bind _asbp_lobby_hud (Utilities|Casting|CastToBP_LobbyHUD (HUD|GetHUD _returnvalue)))
      (Default|RefreshUI _asbp_lobby_hud))))

(fn OnRepNickname
  (CallFunction|RefreshLobbyUI))