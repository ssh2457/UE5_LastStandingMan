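; BP_Stickman is a character that can strike other stickmen and dies from any damage taken while idle, moving or attacking.
; Attack hits run on the authority, sphere-tracing forward for pawns and damaging stickmen; attack end restores the IdleMove state.
; Death is multicast to set Dead and disable movement and capsule collision, then reported to BP_GameMode if the damage causer is a BP_Player.
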(event Custom|Multicast_ProcessDeath
  ;[0.15 0.15 0.15 0.5] Death
  (Utilities|FlowControl|Sequence
    (:then_0
      (Variables|Default|SetState "NewEnumerator2"))
    (:then_1
      (Pawn|Components|CharacterMovement|DisableMovement (Variables|Character|GetCharacterMovement)))
    (:then_2
      (Collision|SetCollisionEnabled (Variables|Collision|GetCapsuleComponent) "NoCollision"))))

(event Game|Damage|EventAnyDamage
  (params (Damage :type Float%20%28single-precision%29) (DamageType :type Damage%20Type%20Object%20Reference) (InstigatedBy :type Controller%20Object%20Reference) (DamageCauser :type Actor%20Object%20Reference))
  ;[0.15 0.15 0.15 0.5] Death
  (switch Utilities|FlowControl|Switch|SwitchonEState (Variables|Default|GetState)
    (:NewEnumerator0
      _)
    (:NewEnumerator1
      _))
  (Utilities|FlowControl|Sequence
    (:then_0
      (CallFunction|MulticastProcessDeath))
    (:then_1
      (bind _asbp_game_mode (Utilities|Casting|CastToBP_GameMode (Game|GetGameMode)))
      (bind _asbp_player (Utilities|Casting|CastToBP_Player DamageCauser))
      (Default|OnStickmanDeath _asbp_game_mode _asbp_player self))))

(event Custom|ProcessAttackHit
  (bind _returnvalue (Transformation|GetActorLocation))
  ;[0.15 0.15 0.15 0.5] Process Battle
  (Networking|SwitchHasAuthority
    (:Authority
      (bind _outhits (Collision|MultiSphereTraceForObjects _returnvalue (+ _returnvalue (* (Transformation|GetActorForwardVector) (Variables|Default|GetAttackRange))) 5e+01 (Utilities|Array|MakeArray "ObjectTypeQuery3") false 0 "None"))
      (for _array_element _outhits
        (bind _asbp_stickman (Utilities|Casting|CastToBP_Stickman (.hitactor _array_element)))
        (Game|Damage|ApplyDamage _asbp_stickman 1.0 0 self)))))

(event Custom|ProcessAttackEnd
  ;[0.15 0.15 0.15 0.5] Process Battle
  (switch Utilities|FlowControl|Switch|SwitchonEState (Variables|Default|GetState)
    (:NewEnumerator1
      (Variables|Default|SetState "NewEnumerator0"))))

(fn ConstructionScript)